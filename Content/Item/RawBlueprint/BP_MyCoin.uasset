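; BP_MyCoin is a coin actor that spins its static mesh and reports when characters enter or leave its sphere.
; Tick yaws the mesh by DeltaSeconds times MoveSpeed for frame-rate independent rotation.
; The sphere's begin and end overlap events filter for Characters and print their display names on screen as debug messages.
; No pickup, scoring or destruction logic is present.
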(event OnComponentBeginOverlap(Sphere)
  (params (OverlappedComponent :type Primitive%20Component%20Object%20Reference) (OtherActor :type Actor%20Object%20Reference) (OtherComp :type Primitive%20Component%20Object%20Reference) (OtherBodyIndex :type Integer) (bFromSweep :type Boolean) (SweepResult :type Hit%20Result%20Structure%20%28by%20ref%29))
  (bind _ascharacter (Utilities|Casting|CastToCharacter OtherActor))
  (Development|PrintString (Utilities|String|Append "BeginOverlap Char : " (Utilities|GetDisplayName _ascharacter)) true true "(R=0.000000,G=0.665387,B=1.000000,A=1.000000)" 6e+01))

(event OnComponentEndOverlap(Sphere)
  (params (OverlappedComponent :type Primitive%20Component%20Object%20Reference) (OtherActor :type Actor%20Object%20Reference) (OtherComp :type Primitive%20Component%20Object%20Reference) (OtherBodyIndex :type Integer))
  (bind _ascharacter (Utilities|Casting|CastToCharacter OtherActor))
  (Development|PrintString (Utilities|String|Append "EndOverlap Char : " (Utilities|GetDisplayName _ascharacter)) true true "(R=0.000000,G=0.665387,B=1.000000,A=1.000000)" 6e+01))

(event EventBeginPlay)

(event Collision|EventActorBeginOverlap
  (params (OtherActor :type Actor%20Object%20Reference)))

(event EventTick
  (params (DeltaSeconds :type Float%20%28single-precision%29))
  (Transformation|AddRelativeRotation (Variables|Default|GetStaticMesh) (Math|Rotator|MakeRotator 0.0 0.0 (* DeltaSeconds (Variables|Default|GetMoveSpeed))) false false))

(fn ConstructionScript)