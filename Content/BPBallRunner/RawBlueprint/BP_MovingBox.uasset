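; BP_MovingBox is an actor that moves itself continuously along local-space offsets, in one of two modes chosen by UseVectorDirection.
; Vector mode moves along a normalized direction each Tick, reversing whenever accumulated travel reaches MaxMoveDistance.
; Enum mode uses a timeline curve to scale speed, switching to the next direction in a fixed six-axis loop each time it finishes.
; Tick also prints the actor's transform as debug output.
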(event Custom|MoveTimeByWorldDirection
  (if (Utilities|Enum|NotEqual(Enum) (Variables|Movement|GetNextMoveDirection) "NewEnumerator2")
    (bind _movetime (Timeline|Timeline_SmoothMoveMent Play)
      (:Update
        (Transformation|AddActorLocalOffset (* (CallFunction|GetMoveDirectionVector (Variables|Movement|GetNextMoveDirection)) (* _movetime (Utilities|Time|GetWorldDeltaSeconds) (Variables|Movement|GetMoveSpeed))) false false))
      (:Finished
        (Variables|Movement|SetNextMoveDirection (Utilities|Select :Index (Variables|Movement|GetNextMoveDirection) :NewEnumerator2 "NewEnumerator2" :NewEnumerator0 "NewEnumerator3" :NewEnumerator1 "NewEnumerator6" :NewEnumerator3 "NewEnumerator4" :NewEnumerator4 "NewEnumerator1" :NewEnumerator5 "NewEnumerator0" :NewEnumerator6 "NewEnumerator5"))
        (Timeline|Timeline_SmoothMoveMent PlayFromStart)))))

(event EventTick
  (params (DeltaSeconds :type Float%20%28single-precision%29))
  (Utilities|FlowControl|Sequence
    (:then_0
      (Development|PrintString (Utilities|String|Append "[" (Utilities|GetDisplayName self) "] Transform : " (Utilities|String|ToString(Transform) (Transformation|GetActorTransform)) "]") true true "(R=0.000000,G=0.660000,B=1.000000,A=1.000000)" DeltaSeconds))
    (:then_1
      (if (Variables|Movement|GetbUseVectorDirection)
        (CallFunction|MoveDirectionFowardNBackward)))))

(event EventBeginPlay
  (if (Variables|Movement|GetbUseVectorDirection)
    ;[1 1 1] Vector방향을 사용할 경우
    (Variables|Movement|SetNextMoveDirection "NewEnumerator2")
    (Variables|Movement|SetNextVectorDirection (Math|Vector|Normalize (Variables|Movement|GetNextVectorDirection)))
    (else
      ;[1 1 1] Enum 방향을 사용할 경우
      (Variables|Movement|SetNextVectorDirection (CallFunction|GetMoveDirectionVector (Variables|Movement|GetNextMoveDirection)))
      (CallFunction|MoveTimebyWorldDirection))))

(fn ConstructionScript)

(fn MoveDirectionFowardNBackward
  (Transformation|AddActorLocalOffset (* (Variables|Movement|GetNextVectorDirection) (* (Utilities|Time|GetWorldDeltaSeconds) (Variables|Movement|GetMoveSpeed))) false false)
  ;[1 1 1] 총 이동거리에 더해준다.
  (Variables|Movement|SetCurMoveDistance (+ (Math|Float|Absolute(Float) (Math|Vector|VectorLength (* (Variables|Movement|GetNextVectorDirection) (* (Utilities|Time|GetWorldDeltaSeconds) (Variables|Movement|GetMoveSpeed))))) (Variables|Movement|GetCurMoveDistance)))
  ;[1 1 1] 최대 제한 이동거리를 초과할 경우
  (if (>= (Variables|Movement|GetCurMoveDistance) (Variables|Movement|GetMaxMoveDistance))
    (Variables|Movement|SetCurMoveDistance 0.0)
    ;[1 1 1] 방향을 반대로 설정한다.
    (Variables|Movement|SetNextVectorDirection (* (Variables|Movement|GetNextVectorDirection) -1.0))))

(fn GetMoveDirectionVector
  (params (EN_MoveDirection :type EN_MoveDirection%20Enum :default "NewEnumerator2"))
  (switch Utilities|FlowControl|Switch|SwitchonEN_MoveDirection EN_MoveDirection
    (:NewEnumerator2
      (LocalVariables|SetOutVector "0, 0, 0"))
    (:NewEnumerator0
      (LocalVariables|SetOutVector "1.000000, 0, 0"))
    (:NewEnumerator1
      (LocalVariables|SetOutVector "-1.000000, 0, 0"))
    (:NewEnumerator3
      (LocalVariables|SetOutVector "0,1.000000, 0"))
    (:NewEnumerator4
      (LocalVariables|SetOutVector "0,-1.000000, 0"))
    (:NewEnumerator5
      (LocalVariables|SetOutVector "0, 0,1.000000"))
    (:NewEnumerator6
      (LocalVariables|SetOutVector "0, 0,-1.000000")))
  (return (LocalVariables|GetOutVector)))