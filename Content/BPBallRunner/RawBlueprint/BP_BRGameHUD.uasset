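; BP_BRGameHUD is the Ball Runner game's HUD, which creates the on-screen UI widget and tracks FPS and elapsed game time.
; On BeginPlay it casts the owning controller to BP_BRPlayerController, retrying on a timer until it succeeds, then adds BP_BRUIWidget to the viewport with a self reference and game-only input.
; Tick updates both values and caches zero-padded string versions of them.
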(event EventBeginPlay
  (CallFunction|BFLPrintLog "HUD BeginPlay!" true true "(R=0.000000,G=1.000000,B=0.000000,A=1.000000)" 6e+01)
  (CallFunction|TryBindPlayerController))

(event EventDrawHUD
  (params (SizeX :type Integer) (SizeY :type Integer)))

(event EventTick
  (params (DeltaSeconds :type Float%20%28single-precision%29))
  (CallFunction|SetCurFPS (/ 1.0 DeltaSeconds))
  (CallFunction|SetElapsedGameTime (+ (Variables|Default|GetElapsedGameTime) (Utilities|Time|GetWorldDeltaSeconds))))

(fn ConstructionScript)

(fn TryBindPlayerController
  (bind _asbp_brplayer_controller (Utilities|Casting|CastToBP_BRPlayerController (Game|Player|GetOwningPlayerController))
    (:then
      (CallFunction|BFLPrintLog "BP_BRHUD_TryBindPlayerController CastSuccess!" true true "(R=0.000000,G=1.000000,B=0.000000,A=1.000000)" 6e+01)
      (Variables|Default|SetPlayerControllerRef _asbp_brplayer_controller)
      (CallFunction|CreateUIWidget))
    (:CastFailed
      (CallFunction|BFLPrintLog "BP_BRHUD_TryBindPlayerController CastFailed!" true true "(R=0.000000,G=1.000000,B=0.000000,A=1.000000)" 6e+01)
      (Utilities|Time|SetTimerbyFunctionName 0 "TryBindPlayerController" 0.1))))

(fn CreateUIWidget
  (bind _returnvalue (UserInterface|CreateWidget "/Game/BPBallRunner/RawBlueprint/BP_BRUIWidget.BP_BRUIWidget_C" 0 self))
  (bind _output_get (Variables|Default|SetUIWidgetRef _returnvalue))
  (UserInterface|Viewport|AddtoViewport _output_get 0)
  (Input|SetInputModeGameOnly (Variables|Default|GetPlayerControllerRef)))

(fn SetCurFPS
  (params (CurFPS :type Float%20%28single-precision%29))
  (bind _output_get (Variables|Default|SetCurFPS CurFPS))
  (Variables|Default|SetCurStrFPS (CallFunction|BFLAddZeroFloatString _output_get 3)))

(fn SetElapsedGameTime
  (params (ElapsedGameTime :type Float%20%28single-precision%29))
  (bind _output_get (Variables|Default|SetElapsedGameTime ElapsedGameTime))
  (Variables|Default|SetCurStrElapsedGameTime (CallFunction|BFLAddZeroFloatString _output_get 6)))