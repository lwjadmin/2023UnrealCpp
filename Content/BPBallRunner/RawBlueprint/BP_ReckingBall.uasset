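; Wrecking ball actor that swings its Scene component like a pendulum, with period, maximum angle and rotation axis set by variables.
; Each Tick, RunAsSinePendulumMotion picks one of two motion functions.
; Sine mode advances a phase angle and sets relative rotation from its sine, resetting each cycle.
; Constant mode adds local rotation at steady speed, covering a quarter-period half arc first, then reversing after each full arc.
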(event EventBeginPlay)

(event EventTick
  (params (DeltaSeconds :type Float%20%28single-precision%29))
  (if (Variables|Movement|GetbRunAsSinePendulumMotion)
    (CallFunction|MoveSinePendulumMotion false DeltaSeconds)
    (else
      (CallFunction|MoveConstantPendulumMotion false DeltaSeconds))))

(fn ConstructionScript)

(fn MoveConstantPendulumMotion
  (params (bUseWorldDeltaSeconds :type Boolean) (Tick :type Float%20%28single-precision%29))
  ;[1 1 0] 1.진자 왕복운동 시간 : PendulumDesiredTimeSec
  ; 2.진자 최대 각도 : PendulumDesiredAngleDeg
  ; 3.현재 진자 각도 : CurrentAngleDeg
  ; 4.진자가 움직일 방향 : DesiredRotationNormal ( 단위벡터처럼 X/Y/Z의 길이가 0또는 1이어야 함)
  ;
  ; 최대 각도가 60도, 진자 왕복운동시간이 4초일 경우
  ; 최초 단 한번 1초에 60도를 찍고, 2초주기로 120도를 찍어야 한다. (사인그래프의 움직임처럼...)
  ; 1초 = (1 / Tick)프레임, 1프레임 = Tick
  (Transformation|AddLocalRotation (Variables|Default|GetScene) (* (Variables|Movement|GetDesiredRotationNormal) (* (/ (select (Variables|ConstantPendulumMotion|GetbReachedDesiredAngleOnce) (* (Variables|Movement|GetPendulumDesiredAngleDeg) 2.0) (Variables|Movement|GetPendulumDesiredAngleDeg)) (select (Variables|ConstantPendulumMotion|GetbReachedDesiredAngleOnce) (/ (Variables|Movement|GetPendulumDesiredTimeSec) 2.0) (/ (Variables|Movement|GetPendulumDesiredTimeSec) 4.0))) (select bUseWorldDeltaSeconds (Utilities|Time|GetWorldDeltaSeconds) Tick))) false false)
  (bind _output_get (Variables|Movement|SetCurrentAngleDeg (+ (Variables|Movement|GetCurrentAngleDeg) (* (/ (select (Variables|ConstantPendulumMotion|GetbReachedDesiredAngleOnce) (* (Variables|Movement|GetPendulumDesiredAngleDeg) 2.0) (Variables|Movement|GetPendulumDesiredAngleDeg)) (select (Variables|ConstantPendulumMotion|GetbReachedDesiredAngleOnce) (/ (Variables|Movement|GetPendulumDesiredTimeSec) 2.0) (/ (Variables|Movement|GetPendulumDesiredTimeSec) 4.0))) (select bUseWorldDeltaSeconds (Utilities|Time|GetWorldDeltaSeconds) Tick)))))
  (if (>= _output_get (select (Variables|ConstantPendulumMotion|GetbReachedDesiredAngleOnce) (* (Variables|Movement|GetPendulumDesiredAngleDeg) 2.0) (Variables|Movement|GetPendulumDesiredAngleDeg)))
    ;[1 1 0] 왕복각도의 끝에 도달할 경우 회전방향을 반대로 하기 위해서 -1을 곱해준다.
    (Variables|ConstantPendulumMotion|SetbReachedDesiredAngleOnce true)
    (Variables|Movement|SetCurrentAngleDeg 0.0)
    (Variables|Movement|SetDesiredRotationNormal (* (Variables|Movement|GetDesiredRotationNormal) -1.0))))

(fn MoveSinePendulumMotion
  (params (bUseWorldDeltaSeconds :type Boolean) (Tick :type Float%20%28single-precision%29))
  (bind _returnvalue (Math|Float|MakeLiteralFloat 3.6e+02))
  ;[1 1 0] 1.진자 왕복운동 시간 : PendulumDesiredTimeSec
  ; 2.진자 최대 각도 : PendulumDesiredAngleDeg
  ; 3.현재 진자 각도 : CurrentAngleDeg
  ; 4.진자가 움직일 방향 : DesiredRotationNormal ( 단위벡터처럼 X/Y/Z의 길이가 0또는 1이어야 함)
  ; 5.Sin함수에 입력할 각도 파라미터 : CurrentThetaDeg
  ;
  ; **진자 왕복운동 시간(PendulumDesiredTimeSec) 내에 CurrentThetaDeg가 360도를 움직여야 한다.
  ; **따라서, 1프레임에 총 몇도가 움직여야 하는지 구해야 한다.
  ;
  ; Ex) 왕복운동시간 = 2초일 경우
  ; 2초에 360도 = 1초에 180도 , 1초 = (1 / Tick)프레임, 1프레임 = Tick
  ; 1프레임당 움직여야 하는 각도(Theta) = 360 / PendulumDesiredTimeSec * Tick
  (bind _output_get (Variables|SinePendulumMotion|SetCurrentThetaDeg (+ (Variables|SinePendulumMotion|GetCurrentThetaDeg) (* (/ _returnvalue (Variables|Movement|GetPendulumDesiredTimeSec)) (Math|Float|SelectFloat (Utilities|Time|GetWorldDeltaSeconds) Tick bUseWorldDeltaSeconds)))))
  (Transformation|SetRelativeRotation (Variables|Default|GetScene) (* (Variables|Movement|GetDesiredRotationNormal) (* (Math|Trig|Sin(Degrees) _output_get) (Variables|Movement|GetPendulumDesiredAngleDeg))) false false)
  ;[1 1 0] 세타값이 무한히 증가할때 Overflow를 방지하기 위해, Sin그래프 주기인 0~360deg범위를 벗어나면 0으로 초기화하도록 했다.
  (Variables|SinePendulumMotion|SetCurrentThetaDeg (select (>= (Variables|SinePendulumMotion|GetCurrentThetaDeg) _returnvalue) 0.0 (Variables|SinePendulumMotion|GetCurrentThetaDeg))))