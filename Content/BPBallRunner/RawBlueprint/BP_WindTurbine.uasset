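; Wind turbine actor that spins its blades and swings its neck back and forth every tick.
; RotateBlade yaws SceneBlade at a speed set in RPM, converted to degrees per second.
; MoveConstantPendulumMotion rotates SceneNeck at constant speed, flipping direction at each limit.
; The first swing covers the desired angle in a quarter period, later swings twice that angle in half a period, keeping the oscillation centered.
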(event EventTick
  (params (DeltaSeconds :type Float%20%28single-precision%29))
  (Utilities|FlowControl|Sequence
    (:then_0
      (CallFunction|RotateBlade false DeltaSeconds))
    (:then_1
      (CallFunction|MoveConstantPendulumMotion false DeltaSeconds))))

(fn ConstructionScript)

(fn MoveConstantPendulumMotion
  (params (bUseWorldDeltaSeconds :type Boolean) (Tick :type Float%20%28single-precision%29))
  ;[1 1 0] 1.진자 왕복운동 시간 : PendulumDesiredTimeSec
  ; 2.진자 최대 각도 : PendulumDesiredAngleDeg
  ; 3.현재 진자 각도 : CurrentAngleDeg
  ; 4.진자가 움직일 방향 : DesiredRotationNormal ( 단위벡터처럼 X/Y/Z의 길이가 0또는 1이어야 함)
  ;
  ; 최대 각도가 60도, 진자 왕복운동시간이 4초일 경우
  ; 최초 단 한번 1초에 60도를 찍고, 2초주기로 120도를 찍어야 한다. (사인그래프의 움직임처럼...)
  ; 1초 = (1 / Tick)프레임, 1프레임 = Tick
  (Transformation|AddLocalRotation (Variables|Default|GetSceneNeck) (* (Variables|ConstantPendulumMotion|GetDesiredRotationNormal) (* (/ (select (Variables|ConstantPendulumMotion|GetbReachedDesiredAngleOnce) (* (Variables|ConstantPendulumMotion|GetPendulumDesiredAngleDeg) 2.0) (Variables|ConstantPendulumMotion|GetPendulumDesiredAngleDeg)) (select (Variables|ConstantPendulumMotion|GetbReachedDesiredAngleOnce) (/ (Variables|ConstantPendulumMotion|GetPendulumDesiredTimeSec) 2.0) (/ (Variables|ConstantPendulumMotion|GetPendulumDesiredTimeSec) 4.0))) (select bUseWorldDeltaSeconds (Utilities|Time|GetWorldDeltaSeconds) Tick))) false false)
  (bind _output_get (Variables|ConstantPendulumMotion|SetCurrentAngleDeg (+ (Variables|ConstantPendulumMotion|GetCurrentAngleDeg) (* (/ (select (Variables|ConstantPendulumMotion|GetbReachedDesiredAngleOnce) (* (Variables|ConstantPendulumMotion|GetPendulumDesiredAngleDeg) 2.0) (Variables|ConstantPendulumMotion|GetPendulumDesiredAngleDeg)) (select (Variables|ConstantPendulumMotion|GetbReachedDesiredAngleOnce) (/ (Variables|ConstantPendulumMotion|GetPendulumDesiredTimeSec) 2.0) (/ (Variables|ConstantPendulumMotion|GetPendulumDesiredTimeSec) 4.0))) (select bUseWorldDeltaSeconds (Utilities|Time|GetWorldDeltaSeconds) Tick)))))
  (if (>= _output_get (select (Variables|ConstantPendulumMotion|GetbReachedDesiredAngleOnce) (* (Variables|ConstantPendulumMotion|GetPendulumDesiredAngleDeg) 2.0) (Variables|ConstantPendulumMotion|GetPendulumDesiredAngleDeg)))
    ;[1 1 0] 왕복각도의 끝에 도달할 경우 회전방향을 반대로 하기 위해서 -1을 곱해준다.
    (Variables|ConstantPendulumMotion|SetbReachedDesiredAngleOnce true)
    (Variables|ConstantPendulumMotion|SetCurrentAngleDeg 0.0)
    (Variables|ConstantPendulumMotion|SetDesiredRotationNormal (* (Variables|ConstantPendulumMotion|GetDesiredRotationNormal) -1.0))))

(fn RotateBlade
  (params (bUseWorldDeltaSeconds :type Boolean) (Tick :type Float%20%28single-precision%29))
  (Transformation|AddRelativeRotation (Variables|Default|GetSceneBlade) (Math|Rotator|MakeRotator 0.0 0.0 (* (select bUseWorldDeltaSeconds (Utilities|Time|GetWorldDeltaSeconds) Tick) (Variables|Movement|GetBladeRotationSpeedRPM) 6.0)) false false))