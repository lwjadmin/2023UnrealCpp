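; BP_BRPlane is a ball runner plane actor whose static mesh shows a configurable grid material.
; Its construction script pushes half of the actor's X and Y scale into the XSize and YSize material parameters, tying the grid to the plane's size.
; It also applies the two grid colors, metallic and roughness variables to the mesh materials.
; The event graph holds no gameplay logic.
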(event EventBeginPlay)

(event Collision|EventActorBeginOverlap
  (params (OtherActor :type Actor%20Object%20Reference)))

(event EventTick
  (params (DeltaSeconds :type Float%20%28single-precision%29)))

(fn ConstructionScript
  (bind _returnvalue (Transformation|GetActorTransform))
  (bind _scale (Math|Transform|BreakTransform _returnvalue))
  (bind (_x _y) (Math|Vector|BreakVector _scale))
  (Utilities|FlowControl|Sequence
    (:then_0
      (Rendering|Material|SetScalarParameterValueonMaterials (Variables|Default|GetStaticMesh) "XSize" (/ _x 2.0))
      (Rendering|Material|SetScalarParameterValueonMaterials (Variables|Default|GetStaticMesh) "YSize" (/ _y 2.0)))
    (:then_1
      (Rendering|Material|SetVectorParameterValueonMaterials (Variables|Default|GetStaticMesh) "GridColor1" (Math|Conversions|ToVector(LinearColor) (Variables|Default|GetGridColor1)))
      (Rendering|Material|SetVectorParameterValueonMaterials (Variables|Default|GetStaticMesh) "GridColor2" (Math|Conversions|ToVector(LinearColor) (Variables|Default|GetGridColor2))))
    (:then_2
      (Rendering|Material|SetScalarParameterValueonMaterials (Variables|Default|GetStaticMesh) "Metalic" (Variables|Default|GetMetalic))
      (Rendering|Material|SetScalarParameterValueonMaterials (Variables|Default|GetStaticMesh) "Roughness" (Variables|Default|GetRoughness)))))