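; Player pawn for a ball runner game: a physics mesh driven by camera-relative forces, with impulse jumps and a smoothly zooming spring-arm camera.
; BeginPlay retries binding BP_BRPlayerState on a timer, then initializes zoom and HP.
; Setters cache transform, speed and HP with formatted strings, firing a death dispatcher at zero HP.
; Hits on Ground re-enable jumping; a Destructable tag on the pawn itself enables speed-based damage.
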(event OnComponentHit(StaticMesh)
  (params (HitComponent :type Primitive%20Component%20Object%20Reference) (OtherActor :type Actor%20Object%20Reference) (OtherComp :type Primitive%20Component%20Object%20Reference) (NormalImpulse :type Vector :default "0, 0, 0") (Hit :type Hit%20Result%20Structure%20%28by%20ref%29))
  (Utilities|FlowControl|Sequence
    (:then_0
      (if (Actor|ActorHasTag OtherActor "Ground")
        (Variables|Default|SetbIsInAir false)))
    (:then_1
      (if (Actor|ActorHasTag "Destructable")
        (Game|Damage|ApplyDamage OtherActor (Variables|Status|GetCurVelocity) 0 self)))))

(event EventBeginPlay
  (CallFunction|BFLPrintLog "Pawn BeginPlay!" true true "(R=0.000000,G=1.000000,B=0.000000,A=1.000000)" 6e+01)
  (CallFunction|TryBindPlayerState))

(event EventTick
  (params (DeltaSeconds :type Float%20%28single-precision%29))
  (CallFunction|SetCurTransform (Transformation|GetActorTransform))
  (CallFunction|SetCurVelocity (Math|Vector|VectorLengthXY (Transformation|GetVelocity)))
  ;[1 1 1] 부드러운 카메라 ZoomIn/ZoomOut
  (Variables|/Script/Engine.SpringArmComponent|SetTargetArmLength (Variables|Default|GetSpringArm) (Math|Interpolation|FInterpTo (Variables|/Script/Engine.SpringArmComponent|GetTargetArmLength (Variables|Default|GetSpringArm)) (Variables|Camera|GetCurSpringArmLength) (Utilities|Time|GetWorldDeltaSeconds) 15.0)))

(event Input|ActionEvents|InputActionJump
  (params (Key :type Key%20Structure :default "None"))
  (:Pressed
    (if (and (not (Variables|Default|GetbIsInAir)) (not (Variables|Status|GetIsDead)))
      (Variables|Default|SetbIsInAir true)
      (Physics|AddImpulse (Variables|Default|GetStaticMesh) (Math|Vector|MakeVector 0.0 0.0 (* (Physics|GetMass (Variables|Default|GetStaticMesh)) (Variables|Movement|GetMeshJumpImpulse))) "None" false))))

(event Input|ActionEvents|InputActionZoomIn
  (params (Key :type Key%20Structure :default "None"))
  (:Pressed
    (Variables|Camera|SetCurSpringArmLength (Math|Float|Clamp(Float) (* (Variables|Camera|GetCurSpringArmLength) 0.95) (Variables|Camera|GetMinSpringArmLength) (Variables|Camera|GetMaxSpringArmLength)))))

(event Input|ActionEvents|InputActionZoomOut
  (params (Key :type Key%20Structure :default "None"))
  (:Pressed
    (Variables|Camera|SetCurSpringArmLength (Math|Float|Clamp(Float) (* (Variables|Camera|GetCurSpringArmLength) 1.05) (Variables|Camera|GetMinSpringArmLength) (Variables|Camera|GetMaxSpringArmLength)))))

(event Input|AxisEvents|InputAxisTurn
  (params (AxisValue :type Float%20%28single-precision%29))
  (Pawn|Input|AddControllerYawInput AxisValue))

(event Input|AxisEvents|InputAxisLookUp
  (params (AxisValue :type Float%20%28single-precision%29))
  (Pawn|Input|AddControllerPitchInput AxisValue))

(event Input|AxisEvents|InputAxisMoveForward
  (params (AxisValue :type Float%20%28single-precision%29))
  (bind _returnvalue (Game|GetPlayerCameraManager 0))
  (bind _meshmovespeed (Variables|Movement|GetMeshMoveSpeed))
  (bind _staticmesh (Variables|Default|GetStaticMesh))
  (bind _returnvalue_2 (Physics|GetMass _staticmesh))
  (bind _returnvalue_3 (Transformation|GetActorForwardVector _returnvalue))
  (bind _returnvalue_4 (* AxisValue _returnvalue_2 _meshmovespeed))
  (bind _returnvalue_5 (* _returnvalue_3 _returnvalue_4))
  (bind (_x _y) (Math|Vector|BreakVector _returnvalue_5))
  (if (not (Variables|Status|GetIsDead))
    (Physics|AddForce (Variables|Default|GetStaticMesh) (Math|Vector|MakeVector _x _y 0.0) "None" false)))

(event Input|AxisEvents|InputAxisMoveRight
  (params (AxisValue :type Float%20%28single-precision%29))
  (bind _returnvalue (Game|GetPlayerCameraManager 0))
  (bind _meshmovespeed (Variables|Movement|GetMeshMoveSpeed))
  (bind _staticmesh (Variables|Default|GetStaticMesh))
  (bind _returnvalue_2 (Physics|GetMass _staticmesh))
  (bind _returnvalue_3 (Transformation|GetActorRightVector _returnvalue))
  (bind _returnvalue_4 (* AxisValue _returnvalue_2 _meshmovespeed))
  (bind _returnvalue_5 (* _returnvalue_3 _returnvalue_4))
  (bind (_x _y) (Math|Vector|BreakVector _returnvalue_5))
  (if (not (Variables|Status|GetIsDead))
    (Physics|AddForce (Variables|Default|GetStaticMesh) (Math|Vector|MakeVector _x _y 0.0) "None" false)))

(fn ConstructionScript)

(fn TryBindPlayerState
  (bind _asbp_brplayer_state (Utilities|Casting|CastToBP_BRPlayerState (Variables|GetPlayerState))
    (:then
      (CallFunction|BFLPrintLog "BRPawn_TryBindPlayerState_BindSuccess!" true true "(R=0.000000,G=1.000000,B=0.000000,A=1.000000)" 6e+01)
      (Variables|Reference|SetPlayerStateRef _asbp_brplayer_state)
      (CallFunction|InitPawn))
    (:CastFailed
      (CallFunction|BFLPrintLog "BRPawn_TryBindPlayerState_BindFail!" true true "(R=0.000000,G=1.000000,B=0.000000,A=1.000000)" 6e+01)
      (Utilities|Time|SetTimerbyFunctionName 0 "TryBindPlayerState" 0.1))))

(fn InitPawn
  (bind _output_get (Variables|Camera|SetMaxSpringArmLength (Variables|/Script/Engine.SpringArmComponent|GetTargetArmLength (Variables|Default|GetSpringArm))))
  (Variables|Camera|SetCurSpringArmLength _output_get)
  (Variables|Status|SetCurTransform (Transformation|GetActorTransform))
  (CallFunction|SetMaxHP 1e+02)
  (CallFunction|SetCurHP (Variables|Status|GetMaxHP)))

(fn SetCurTransform
  (params (NewTransform :type Transform))
  (bind _output_get (Variables|Status|SetCurTransform NewTransform))
  (Variables|Status|SetCurStrPosition (CallFunction|BFLVectortoString (.Location (Math|Transform|BreakTransform _output_get)) 5)))

(fn SetCurVelocity
  (params (NewVelocity :type Float%20%28single-precision%29))
  (bind _output_get (Variables|Status|SetCurVelocity NewVelocity))
  (Variables|Status|SetCurStrVelocity (CallFunction|BFLAddZeroFloatString _output_get 4)))

(fn SetCurHP
  (params (CurHP :type Float%20%28single-precision%29))
  (bind _output_get (Variables|Status|SetCurHP (Math|Float|Clamp(Float) CurHP 0.0 (Variables|Status|GetMaxHP))))
  (Variables|Status|SetStrCurHP (CallFunction|BFLAddZeroFloatString _output_get 3))
  (bind _output_get_2 (Variables|Status|SetIsDead (== _output_get 0.0)))
  (if _output_get_2
    (Default|CallEventDispatcherPlayerDead)))

(fn SetMaxHP
  (params (MaxHP :type Float%20%28single-precision%29))
  (bind _output_get (Variables|Status|SetMaxHP MaxHP))
  (Variables|Status|SetStrMaxHP (CallFunction|BFLAddZeroFloatString _output_get 3)))