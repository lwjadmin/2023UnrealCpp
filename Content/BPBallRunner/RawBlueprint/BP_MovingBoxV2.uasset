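; BP_MovingBoxV2 is an actor that moves in a straight line from its spawn location to a configurable offset.
; Tick moves it at MoveSpeed without sweeping, accumulating travelled distance to detect arrival and snap to the target.
; It then either swaps endpoints for a round trip or collapses them so movement stops.
; An optional debug line shows the path, redrawn by a repeating timer.
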(event EventBeginPlay
  (Variables|Movement|SetBaseWorldLocation (Transformation|GetActorLocation))
  (Variables|Movement|SetNextWorldLocation (+ (Variables|Movement|GetNextLocalLocation) (Variables|Movement|GetBaseWorldLocation)))
  (CallFunction|ShowDebugLine))

(event EventTick
  (params (DeltaSeconds :type Float%20%28single-precision%29))
  (CallFunction|MoveVectorDirection false DeltaSeconds))

(fn ConstructionScript)

(fn ShowDebugLine
  (if (Variables|Default|GetbShowDebugLine)
    (Rendering|Debug|DrawDebugLine (Variables|Movement|GetBaseWorldLocation) (Variables|Movement|GetNextWorldLocation) "(R=1.000000,G=0.000000,B=0.000000,A=1.000000)" 5.0 1.0)
    (Utilities|Time|SetTimerbyFunctionName 0 "ShowDebugLine" 5.0)))

(fn MoveVectorDirection
  (params (bUseWorldDeltaSeconds :type Boolean) (Tick :type Float%20%28single-precision%29))
  (if (> (Math|Vector|VectorLength (* (Math|Vector|Normalize (- (Variables|Movement|GetNextWorldLocation) (Variables|Movement|GetBaseWorldLocation))) (* (Variables|Movement|GetMoveSpeed) (Math|Float|SelectFloat (Utilities|Time|GetWorldDeltaSeconds) Tick bUseWorldDeltaSeconds)))) 0.0)
    (bind _output_get (Variables|Movement|SetTotalMoveDistance (+ (Math|Vector|VectorLength (* (Math|Vector|Normalize (- (Variables|Movement|GetNextWorldLocation) (Variables|Movement|GetBaseWorldLocation))) (* (Variables|Movement|GetMoveSpeed) (Math|Float|SelectFloat (Utilities|Time|GetWorldDeltaSeconds) Tick bUseWorldDeltaSeconds)))) (Variables|Movement|GetTotalMoveDistance))))
    (if (>= _output_get (Math|Vector|Distance(Vector) (Variables|Movement|GetNextWorldLocation) (Variables|Movement|GetBaseWorldLocation)))
      (Transformation|SetActorLocation (Variables|Movement|GetNextWorldLocation) false false)
      (if (Variables|Movement|GetbMoveRoundTrip)
        (Variables|Movement|SetTotalMoveDistance 0.0)
        (Variables|Movement|SetTempLocation (Variables|Movement|GetBaseWorldLocation))
        (Variables|Movement|SetBaseWorldLocation (Variables|Movement|GetNextWorldLocation))
        (Variables|Movement|SetNextWorldLocation (Variables|Movement|GetTempLocation))
        (else
          (Variables|Movement|SetBaseWorldLocation (Variables|Movement|GetNextWorldLocation))))
      (else
        (Transformation|AddActorWorldOffset (* (Math|Vector|Normalize (- (Variables|Movement|GetNextWorldLocation) (Variables|Movement|GetBaseWorldLocation))) (* (Variables|Movement|GetMoveSpeed) (Math|Float|SelectFloat (Utilities|Time|GetWorldDeltaSeconds) Tick bUseWorldDeltaSeconds))))))))