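; BP_MovingBoxV3 is a box actor that draws a debug preview of a waypoint path; it contains no movement logic itself.
; Its construction script sets base color, roughness and metallic material parameters, optionally randomizing them.
; BeginPlay stores the world location as the base for NextLocalLocationList offsets and calls ShowDebugLine.
; That function draws numbered red points joined by arrows, then sets a timer on itself by name.
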(event EventBeginPlay
  (Variables|Default|SetBaseWorldLocation (Transformation|GetActorLocation))
  (CallFunction|ShowDebugLine true))

(event Collision|EventActorBeginOverlap
  (params (OtherActor :type Actor%20Object%20Reference)))

(event EventTick
  (params (DeltaSeconds :type Float%20%28single-precision%29)))

(fn ConstructionScript
  (Utilities|FlowControl|Sequence
    (:then_0
      (bind _output_get (Variables|Outfit|SetMeshBaseColor (Math|Color|SelectColor (Math|Color|MakeColor (Math|Random|RandomFloatinRange 0.2 1.0) (Math|Random|RandomFloatinRange 0.2 1.0) (Math|Random|RandomFloatinRange 0.2 1.0)) (Variables|Outfit|GetMeshBaseColor) (Variables|Outfit|GetbSetRandomizedMaterial))))
      (Rendering|Material|SetVectorParameterValueonMaterials (Variables|Default|GetStaticMesh) "BaseColor" (Math|Conversions|ToVector(LinearColor) _output_get)))
    (:then_1
      (Variables|Outfit|SetRoughness (select (Variables|Outfit|GetbSetRandomizedMaterial) (Math|Random|RandomFloatinRange 0.2 0.8) (Variables|Outfit|GetRoughness)))
      (Rendering|Material|SetScalarParameterValueonMaterials (Variables|Default|GetStaticMesh) "Roughness" (select (Variables|Outfit|GetbSetRandomizedMaterial) (Math|Random|RandomFloatinRange 0.2 0.8) (Variables|Outfit|GetRoughness))))
    (:then_2
      (Variables|Outfit|SetMetalic (select (Variables|Outfit|GetbSetRandomizedMaterial) (Math|Random|RandomFloatinRange 0.0 0.2) (Variables|Outfit|GetMetalic)))
      (Rendering|Material|SetScalarParameterValueonMaterials (Variables|Default|GetStaticMesh) "Metalic" (select (Variables|Outfit|GetbSetRandomizedMaterial) (Math|Random|RandomFloatinRange 0.0 0.2) (Variables|Outfit|GetMetalic))))))

(fn ShowDebugLine
  (params (bShowDebugLine :type Boolean))
  (LocalVariables|SetPrevVector (Transformation|GetActorLocation))
  (if bShowDebugLine
    (for (_array_element _array_index) (Variables|Movement|GetNextLocalLocationList)
      (Rendering|Debug|DrawDebugArrow (LocalVariables|GetPrevVector) (+ (Variables|Default|GetBaseWorldLocation) _array_element) 3e+01 "(R=1.000000,G=0.000000,B=0.000000,A=1.000000)" 6e+01 1.0)
      (bind _output_get (LocalVariables|SetPrevVector (+ (Variables|Default|GetBaseWorldLocation) _array_element)))
      (Rendering|Debug|DrawDebugPoint _output_get 1e+01 "(R=1.000000,G=0.000000,B=0.000000,A=1.000000)" 6e+01)
      (Rendering|Debug|DrawDebugString (+ _output_get "0.000000,0.000000,-10.000000") (Utilities|String|ToString(Integer) (+ _array_index 1)) 0 "(R=1.000000,G=0.000000,B=0.000000,A=1.000000)" 6e+01))
    (Utilities|Time|SetTimerbyFunctionName 0 "ShowDebugLine" 6e+01)))