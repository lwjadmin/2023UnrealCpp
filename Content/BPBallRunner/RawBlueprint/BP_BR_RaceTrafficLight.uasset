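; Race start traffic light Blueprint with five sphere lamps: one red, three yellow and one green.
; The construction script sets lamp colors with emissive off, and PowerOn lights the red lamp.
; LightsOn uses a delayed-loop macro to light the remaining lamps one second apart, while LightsOff resets to red only.
; Lamps switch through material EmissiveIntensity, and keys 1, 2 and 3 trigger PowerOn, LightsOn and LightsOff.
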(event EventBeginPlay
  (Variables|Lights|SetLightsArray (Utilities|Array|MakeArray (Variables|Default|GetSphere1) (Variables|Default|GetSphere2) (Variables|Default|GetSphere3) (Variables|Default|GetSphere4) (Variables|Default|GetSphere5)))
  (Input|EnableInput (Game|GetPlayerController 0)))

(event EventLightsOff
  (for _array_element (Variables|Lights|GetLightsArray)
    (CallFunction|LightsOffSingleLight _array_element)
    (CallFunction|LightsonSingleLight (Utilities|Array|Get(acopy) (Variables|Lights|GetLightsArray)))))

(event EventLightson
  (bind _index (Utilities|BMLforLoopwithDelay 1 (- (Utilities|Array|Length (Variables|Lights|GetLightsArray)) 1) 1.0)
    (:Loop%20Body
      (CallFunction|LightsonSingleLight (Utilities|Array|Get(acopy) (Variables|Lights|GetLightsArray) _index)))))

(event Input|KeyboardEvents|1
  (params (Key :type Key%20Structure :default "None"))
  (:Pressed
    (CallFunction|Poweron)))

(event Input|KeyboardEvents|2
  (params (Key :type Key%20Structure :default "None"))
  (:Pressed
    (CallFunction|Lightson)))

(event Input|KeyboardEvents|3
  (params (Key :type Key%20Structure :default "None"))
  (:Pressed
    (CallFunction|LightsOff)))

(fn ConstructionScript
  (CallFunction|PowerOff))

(fn Poweron
  (Variables|Lights|SetIsPowerOn true)
  (Rendering|Material|SetVectorParameterValueonMaterials (Variables|Default|GetSphere2) "BaseColor" (Math|Conversions|ToVector(LinearColor) (Math|Color|MakeColor 1.0 1.0 0.0)))
  (Rendering|Material|SetVectorParameterValueonMaterials (Variables|Default|GetSphere5) "BaseColor" (Math|Conversions|ToVector(LinearColor) (Math|Color|MakeColor 0.0 1.0 0.0)))
  (Rendering|Material|SetVectorParameterValueonMaterials (Variables|Default|GetSphere1) "BaseColor" (Math|Conversions|ToVector(LinearColor) (Math|Color|MakeColor 1.0 0.0 0.0)))
  (Rendering|Material|SetScalarParameterValueonMaterials (Variables|Default|GetSphere1) "EmissiveIntensity" (Variables|Lights|GetEmissiveIntensity)))

(fn PowerOff
  (Rendering|Material|SetVectorParameterValueonMaterials (Variables|Default|GetSphere2) "BaseColor" (Math|Conversions|ToVector(LinearColor) (Math|Color|MakeColor 1.0 1.0 0.0)))
  (Rendering|Material|SetVectorParameterValueonMaterials (Variables|Default|GetSphere5) "BaseColor" (Math|Conversions|ToVector(LinearColor) (Math|Color|MakeColor 0.0 1.0 0.0)))
  (Rendering|Material|SetVectorParameterValueonMaterials (Variables|Default|GetSphere1) "BaseColor" (Math|Conversions|ToVector(LinearColor) (Math|Color|MakeColor 1.0 0.0 0.0)))
  (Rendering|Material|SetScalarParameterValueonMaterials (Variables|Default|GetSphere1) "EmissiveIntensity" 0.0)
  (Variables|Lights|SetIsPowerOn false))

(fn LightsonSingleLight
  (params (StaticMeshComponent :type Static%20Mesh%20Component%20Object%20Reference))
  (Rendering|Material|SetScalarParameterValueonMaterials StaticMeshComponent "EmissiveIntensity" (Variables|Lights|GetEmissiveIntensity)))

(fn LightsOffSingleLight
  (params (StaticMeshComponent :type Static%20Mesh%20Component%20Object%20Reference))
  (Rendering|Material|SetScalarParameterValueonMaterials StaticMeshComponent "EmissiveIntensity" 0.0))