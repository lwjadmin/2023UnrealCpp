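; BP_BRTimer is a timer for BallRunner that counts elapsed time and shows it in whole seconds on a TextRender component.
; Tick accumulates delta seconds, truncates the total and compares it as a string to the cached PrevString, so the text updates only when the second changes.
; Each change is also printed on screen as a long-lived debug string.
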(event EventTick
  (params (DeltaSeconds :type Float%20%28single-precision%29))
  (bind _output_get (Variables|Default|SetElapsedTime (+ (Variables|Default|GetElapsedTime) DeltaSeconds)))
  (if (Utilities|Enum|NotEqual(Enum) (Variables|Default|GetPrevString) (Utilities|String|ToString(Integer) (Math|Float|Truncate _output_get)))
    (bind _output_get_2 (Variables|Default|SetPrevString (Utilities|String|ToString(Integer) (Math|Float|Truncate _output_get))))
    (Rendering|Components|TextRender|SetText (Variables|Default|GetTextRender) (Utilities|Text|ToText(String) _output_get_2))
    (Development|PrintString _output_get_2 true true "(R=0.000000,G=0.660000,B=1.000000,A=1.000000)" 6e+01)))

(fn ConstructionScript)