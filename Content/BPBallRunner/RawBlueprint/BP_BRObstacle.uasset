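; BP_BRObstacle is a destructible obstacle for the Ball Runner game, tagged as both Ground and Destructable at BeginPlay.
; Any damage applies a radial force to its DestructibleMesh from the actor's location, with strength equal to the damage amount.
; The construction script feeds half the actor's X/Y scale into the grid material's size parameters, along with its two grid colors, metallic and roughness values.
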(event EventBeginPlay
  (Variables|Default|SetTags self (Utilities|Array|MakeArray "Ground" "Destructable")))

(event Collision|EventActorBeginOverlap
  (params (OtherActor :type Actor%20Object%20Reference)))

(event EventTick
  (params (DeltaSeconds :type Float%20%28single-precision%29)))

(event Game|Damage|EventAnyDamage
  (params (Damage :type Float%20%28single-precision%29) (DamageType :type Damage%20Type%20Object%20Reference) (InstigatedBy :type Controller%20Object%20Reference) (DamageCauser :type Actor%20Object%20Reference))
  (Physics|AddRadialForce (Variables|Default|GetDestructibleMesh) (Transformation|GetActorLocation) 5e+02 Damage "RIF_Constant" false))

(event Collision|EventHit
  (params (MyComp :type Primitive%20Component%20Object%20Reference) (Other :type Actor%20Object%20Reference) (OtherComp :type Primitive%20Component%20Object%20Reference) (bSelfMoved :type Boolean) (HitLocation :type Vector :default "0, 0, 0") (HitNormal :type Vector :default "0, 0, 0") (NormalImpulse :type Vector :default "0, 0, 0") (Hit :type Hit%20Result%20Structure%20%28by%20ref%29)))

(fn ConstructionScript
  (bind _returnvalue (Transformation|GetActorTransform))
  (bind _scale (Math|Transform|BreakTransform _returnvalue))
  (bind (_x _y) (Math|Vector|BreakVector _scale))
  (Utilities|FlowControl|Sequence
    (:then_0
      (Rendering|Material|SetScalarParameterValueonMaterials (Variables|Default|GetDestructibleMesh) "XSize" (/ _x 2.0))
      (Rendering|Material|SetScalarParameterValueonMaterials (Variables|Default|GetDestructibleMesh) "YSize" (/ _y 2.0)))
    (:then_1
      (Rendering|Material|SetVectorParameterValueonMaterials (Variables|Default|GetDestructibleMesh) "GridColor1" (Math|Conversions|ToVector(LinearColor) (Variables|Default|GetGridColor1)))
      (Rendering|Material|SetVectorParameterValueonMaterials (Variables|Default|GetDestructibleMesh) "GridColor2" (Math|Conversions|ToVector(LinearColor) (Variables|Default|GetGridColor2))))
    (:then_2
      (Rendering|Material|SetScalarParameterValueonMaterials (Variables|Default|GetDestructibleMesh) "Metalic" (Variables|Default|GetMetalic))
      (Rendering|Material|SetScalarParameterValueonMaterials (Variables|Default|GetDestructibleMesh) "Roughness" (Variables|Default|GetRoughness)))))