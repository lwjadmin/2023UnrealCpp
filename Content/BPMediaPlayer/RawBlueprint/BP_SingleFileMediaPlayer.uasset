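; Actor that plays a single media source through a Media Player, with sound on MediaSound and a PlaneScreen whose material reflects source validity.
; BeginPlay opens the source with autoplay and loop options, and events control playback, seeking, volume, mute and rate.
; Without autoplay, and on stop, it rewinds, plays briefly and pauses, with a flag preventing that delayed pause from interrupting PlayTrack.
; Tick prints elapsed and total time on screen.
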(event Custom|IgniteMediaPlayer
  (bind _targetmediaplayer (Variables|MediaPlayer|GetTargetMediaPlayer))
  (if (Variables|MediaPlayer|GetIsValidSource)
    (Class|MediaPlayer|Rewind _targetmediaplayer)
    (Media|MediaPlayer|Play _targetmediaplayer :!class /Script/MediaAssets.MediaPlayer)
    (Utilities|FlowControl|Delay 0.5)
    (if (not (Variables|MediaPlayer|GetPlayTrackCalled))
      (Sequencer|Player|Pause _targetmediaplayer)
      (Variables|MediaPlayer|SetIsPlaying false))))

(event EventBeginPlay
  (bind _targetmediasource (Variables|MediaPlayer|GetTargetMediaSource))
  (bind _targetmediaplayer (Variables|MediaPlayer|GetTargetMediaPlayer))
  (if (and (Utilities|IsValid _targetmediaplayer) (Utilities|IsValid _targetmediasource))
    (Media|MediaSoundComponent|SetMediaPlayer (Variables|Default|GetMediaSound) _targetmediaplayer)
    (Media|MediaPlayer|BindEventtoOnMediaOpened _targetmediaplayer (EventDispatchers|CreateEvent :!event OnMediaOpenSuccess))
    (Media|MediaPlayer|BindEventtoOnMediaOpenFailed _targetmediaplayer (EventDispatchers|CreateEvent :!event OnMediaOpenFailed))
    (Media|MediaPlayer|OpenSourcewithOptions _targetmediaplayer _targetmediasource (Utilities|Struct|MakeMediaPlayerOptions "(Audio=0,Caption=-1,Metadata=-1,Script=-1,Subtitle=-1,Text=-1,Video=0)" "+00000000.00:00:00.000000000" (select (Variables|MediaPlayer|GetEnableAutoPlay) "Enabled" "Disabled") (select (Variables|MediaPlayer|GetEnableLooping) "Enabled" "Disabled")) :!class /Script/MediaAssets.MediaPlayer)))

(event EventIncreasePlayRate
  (bind _output_get (Variables|MediaPlayer|SetCurrentPlayRate (Math|Float|Clamp(Float) (+ (Variables|MediaPlayer|GetCurrentPlayRate) 0.1) 0.5 1.5)))
  (Class|MediaPlayer|SetRate (Variables|MediaPlayer|GetTargetMediaPlayer) _output_get))

(event EventMuteVolume
  (bind _output_get (Variables|MediaPlayer|SetIsMute true))
  (Audio|Components|Audio|SetVolumeMultiplier (Variables|Default|GetMediaSound) (Math|Float|SelectFloat 0.0 (Variables|MediaPlayer|GetCurrentVolume) _output_get) :!class /Script/AudioMixer.SynthComponent))

(event EventSetDefaultVolume
  (bind _output_get (Variables|MediaPlayer|SetIsMute false))
  (Audio|Components|Audio|SetVolumeMultiplier (Variables|Default|GetMediaSound) (Math|Float|SelectFloat 0.0 (Variables|MediaPlayer|GetCurrentVolume) _output_get) :!class /Script/AudioMixer.SynthComponent))

(event EventSetDefaultPlayRate
  (bind _output_get (Variables|MediaPlayer|SetCurrentPlayRate 1.0))
  (Class|MediaPlayer|SetRate (Variables|MediaPlayer|GetTargetMediaPlayer) _output_get))

(event EventTick
  (params (DeltaSeconds :type Float%20%28single-precision%29))
  (bind _targetmediaplayer (Variables|MediaPlayer|GetTargetMediaPlayer))
  (Development|PrintString (Utilities|String|Append (CallFunction|BFLTotalSecondstoString (Math|Timespan|GetTotalSeconds (Class|MediaPlayer|GetTime _targetmediaplayer))) "/" (CallFunction|BFLTotalSecondstoString (Math|Timespan|GetTotalSeconds (Media|MediaPlayer|GetDuration _targetmediaplayer)))) true true "(R=0.000000,G=0.660000,B=1.000000,A=1.000000)" DeltaSeconds))

(event EventSeekDirectPlayback
  (params (SeekPercent :type Float%20%28single-precision%29))
  (bind _targetmediaplayer (Variables|MediaPlayer|GetTargetMediaPlayer))
  (Sequencer|Player|Pause _targetmediaplayer)
  (Media|MediaPlayer|Seek _targetmediaplayer (CallFunction|BFLTotalSecondstoTimeSpan (* SeekPercent (/ (Math|Timespan|GetTotalSeconds (Media|MediaPlayer|GetDuration _targetmediaplayer)) 1e+02))))
  (bind _returnvalue (Media|MediaPlayer|Play _targetmediaplayer :!class /Script/MediaAssets.MediaPlayer))
  (Variables|MediaPlayer|SetIsPlaying _returnvalue))

(event EventDecreasePlayRate
  (bind _output_get (Variables|MediaPlayer|SetCurrentPlayRate (Math|Float|Clamp(Float) (- (Variables|MediaPlayer|GetCurrentPlayRate) 0.1) 0.5 1.5)))
  (Class|MediaPlayer|SetRate (Variables|MediaPlayer|GetTargetMediaPlayer) _output_get))

(event EventPlayTrack
  ;[1 1 0] Ignite Delay 중 PlayTrack시, Pause에 의해 끊김방지를 위해 추가함
  (Variables|MediaPlayer|SetPlayTrackCalled true)
  (if (and (Variables|MediaPlayer|GetIsValidSource) (not (Variables|MediaPlayer|GetIsPlaying)))
    (Media|MediaPlayer|Play (Variables|MediaPlayer|GetTargetMediaPlayer) :!class /Script/MediaAssets.MediaPlayer)
    (Variables|MediaPlayer|SetIsPlaying true)))

(event EventStopTrack
  (Variables|MediaPlayer|SetPlayTrackCalled false)
  (if (and (Variables|MediaPlayer|GetIsValidSource) true)
    (Variables|MediaPlayer|SetIsPlaying false)
    (CallFunction|IgniteMediaPlayer)))

(event EventSeekForwardPlayback
  (bind _targetmediaplayer (Variables|MediaPlayer|GetTargetMediaPlayer))
  (bind _returnvalue (Class|MediaPlayer|GetTime _targetmediaplayer))
  (bind (_days _hours _minutes _seconds _milliseconds) (Math|Timespan|BreakTimespan _returnvalue))
  (Sequencer|Player|Pause _targetmediaplayer)
  (Media|MediaPlayer|Seek _targetmediaplayer (Math|Timespan|MakeTimespan _days _hours _minutes (+ _seconds (Variables|MediaPlayer|GetSeekIntervalSecond)) _milliseconds))
  (bind _returnvalue_2 (Media|MediaPlayer|Play _targetmediaplayer :!class /Script/MediaAssets.MediaPlayer))
  (Variables|MediaPlayer|SetIsPlaying _returnvalue_2))

(event EventSeekReversePlayback
  (bind _targetmediaplayer (Variables|MediaPlayer|GetTargetMediaPlayer))
  (bind _returnvalue (Class|MediaPlayer|GetTime _targetmediaplayer))
  (bind (_days _hours _minutes _seconds _milliseconds) (Math|Timespan|BreakTimespan _returnvalue))
  (Sequencer|Player|Pause _targetmediaplayer)
  (Media|MediaPlayer|Seek _targetmediaplayer (Math|Timespan|MakeTimespan _days _hours _minutes (- _seconds (Variables|MediaPlayer|GetSeekIntervalSecond)) _milliseconds))
  (bind _returnvalue_2 (Media|MediaPlayer|Play _targetmediaplayer :!class /Script/MediaAssets.MediaPlayer))
  (Variables|MediaPlayer|SetIsPlaying _returnvalue_2))

(event EventIncreaseVolume
  (bind _output_get (Variables|MediaPlayer|SetCurrentVolume (Math|Float|Clamp(Float) (+ (Variables|MediaPlayer|GetCurrentVolume) 0.1))))
  (Audio|Components|Audio|SetVolumeMultiplier (Variables|Default|GetMediaSound) _output_get :!class /Script/AudioMixer.SynthComponent))

(event EventDecreaseVolume
  (bind _output_get (Variables|MediaPlayer|SetCurrentVolume (Math|Float|Clamp(Float) (- (Variables|MediaPlayer|GetCurrentVolume) 0.1))))
  (Audio|Components|Audio|SetVolumeMultiplier (Variables|Default|GetMediaSound) _output_get :!class /Script/AudioMixer.SynthComponent))

(event EventPauseTrack
  (Variables|MediaPlayer|SetPlayTrackCalled false)
  (if (and (Variables|MediaPlayer|GetIsValidSource) (Variables|MediaPlayer|GetIsPlaying))
    (Sequencer|Player|Pause (Variables|MediaPlayer|GetTargetMediaPlayer))
    (Variables|MediaPlayer|SetIsPlaying false)))

(fn ConstructionScript)

(fn OnMediaOpenSuccess
  (params (OpenedUrl :type String))
  (Development|PrintString (Utilities|String|Append (Utilities|String|Append (Utilities|GetDisplayName self) "::MediaPlayer") "::MediaOpenSuccess, FileURL : " OpenedUrl) true true "(R=0.000000,G=0.660000,B=1.000000,A=1.000000)" 6e+01)
  (bind _output_get (Variables|MediaPlayer|SetIsValidSource true))
  (Rendering|Material|SetScalarParameterValueonMaterials (Variables|Default|GetPlaneScreen) "bIsValidSource" (Math|Conversions|ToFloat(Boolean) _output_get))
  (bind _output_get_2 (Variables|MediaPlayer|SetIsPlaying (Variables|MediaPlayer|GetEnableAutoPlay)))
  (if (not _output_get_2)
    (CallFunction|IgniteMediaPlayer)))

(fn OnMediaOpenFailed
  (params (FailedUrl :type String))
  (Development|PrintString (Utilities|String|Append (Utilities|String|Append (Utilities|GetDisplayName self) "::MediaPlayer") "::MediaOpenFailed, FileURL : " FailedUrl) true true "(R=0.000000,G=0.660000,B=1.000000,A=1.000000)" 6e+01)
  (bind _output_get (Variables|MediaPlayer|SetIsValidSource false))
  (Rendering|Material|SetScalarParameterValueonMaterials (Variables|Default|GetPlaneScreen) "bIsValidSource" (Math|Conversions|ToFloat(Boolean) _output_get))
  (Variables|MediaPlayer|SetIsPlaying false))