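; Player pawn that serves as a keyboard and camera controller for a target media player.
; Look axes rotate the controller, and zoom actions scale the camera's field of view within clamped limits.
; Hard-coded keys forward play/pause, stop, seek, volume, mute and play rate commands to TargetMediaPlayer, with validity checks on only some.
; BeginPlay is empty, and the UI widget creation and input mode setup is unconnected, so it never runs.
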(event EventBeginPlay)

(event Input|ActionEvents|InputActionZoomIn
  (params (Key :type Key%20Structure))
  (:Pressed
    (Camera|SetFieldOfView (Variables|Default|GetCamera) (Math|Float|Clamp(Float) (* (Variables|/Script/Engine.CameraComponent|GetFieldOfView (Variables|Default|GetCamera)) 0.95) 75.0 125.0))))

(event Input|ActionEvents|InputActionZoomOut
  (params (Key :type Key%20Structure))
  (:Pressed
    (Camera|SetFieldOfView (Variables|Default|GetCamera) (Math|Float|Clamp(Float) (* (Variables|/Script/Engine.CameraComponent|GetFieldOfView (Variables|Default|GetCamera)) 1.05) 75.0 125.0))))

(event Input|AxisEvents|InputAxisLookUp
  (params (AxisValue :type Float%20%28single-precision%29))
  (Pawn|Input|AddControllerPitchInput AxisValue))

(event Input|AxisEvents|InputAxisTurn
  (params (AxisValue :type Float%20%28single-precision%29))
  (Pawn|Input|AddControllerYawInput AxisValue))

(event Input|KeyboardEvents|SpaceBar
  (params (Key :type Key%20Structure))
  (bind _targetmediaplayer (Variables|Default|GetTargetMediaPlayer))
  (:Pressed
    (if (Variables|/Game/BPMediaPlayer/RawBlueprint/BP_SingleFileMediaPlayer.BP_SingleFileMediaPlayer_C|GetIsPlaying _targetmediaplayer)
      (Class|BPIMediaPlayer|PauseTrack(Message) _targetmediaplayer)
      (else
        (Class|BPIMediaPlayer|PlayTrack(Message) _targetmediaplayer)))))

(event Input|KeyboardEvents|Right
  (params (Key :type Key%20Structure))
  (bind _targetmediaplayer (Variables|Default|GetTargetMediaPlayer))
  (:Pressed
    (Utilities|IsValid _targetmediaplayer
      (:Is%20Valid
        (if true
          (Class|BPIMediaPlayer|SeekForwardPlayback(Message) _targetmediaplayer))))))

(event Input|KeyboardEvents|Left
  (params (Key :type Key%20Structure))
  (bind _targetmediaplayer (Variables|Default|GetTargetMediaPlayer))
  (:Pressed
    (Utilities|IsValid _targetmediaplayer
      (:Is%20Valid
        (if true
          (Class|BPIMediaPlayer|SeekReversePlayback(Message) _targetmediaplayer))))))

(event Input|KeyboardEvents|Up
  (params (Key :type Key%20Structure))
  (bind _targetmediaplayer (Variables|Default|GetTargetMediaPlayer))
  (:Pressed
    (Utilities|IsValid _targetmediaplayer
      (:Is%20Valid
        (Class|BPIMediaPlayer|IncreaseVolume(Message) _targetmediaplayer)))))

(event Input|KeyboardEvents|Down
  (params (Key :type Key%20Structure))
  (bind _targetmediaplayer (Variables|Default|GetTargetMediaPlayer))
  (:Pressed
    (Utilities|IsValid _targetmediaplayer
      (:Is%20Valid
        (Default|DecreaseVolume _targetmediaplayer)))))

(event Input|KeyboardEvents|M
  (params (Key :type Key%20Structure))
  (bind _targetmediaplayer (Variables|Default|GetTargetMediaPlayer))
  (:Pressed
    (Utilities|IsValid _targetmediaplayer
      (:Is%20Valid
        (if (Variables|/Game/BPMediaPlayer/RawBlueprint/BP_SingleFileMediaPlayer.BP_SingleFileMediaPlayer_C|GetIsMute _targetmediaplayer)
          (Default|SetDefaultVolume _targetmediaplayer)
          (else
            (Default|MuteVolume _targetmediaplayer)))))))

(event Input|KeyboardEvents|Q
  (params (Key :type Key%20Structure))
  (:Pressed
    (Default|StopTrack (Variables|Default|GetTargetMediaPlayer))))

(event Input|KeyboardEvents|Z
  (params (Key :type Key%20Structure))
  (:Pressed
    (Class|BPIMediaPlayer|SetDefaultPlayRate(Message) (Variables|Default|GetTargetMediaPlayer))))

(event Input|KeyboardEvents|X
  (params (Key :type Key%20Structure))
  (:Pressed
    (Default|DecreasePlayRate (Variables|Default|GetTargetMediaPlayer))))

(event Input|KeyboardEvents|C
  (params (Key :type Key%20Structure))
  (:Pressed
    (Default|IncreasePlayRate (Variables|Default|GetTargetMediaPlayer))))

(fn ConstructionScript)